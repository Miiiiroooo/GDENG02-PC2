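; Breakable red fractured mesh that counts hits from BP_PC2_Bullet and releases a random drop when broken.
; A bullet hit increments NHit while it is below three; a hit at exactly three spawns an ExplosionField at the actor's location, guarded by a one-time Break flag.
; It also spawns one of four drop Blueprints there and sets itself as ParentActor on that drop's DropBehaviorActorComponent.
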(event EventBeginPlay)

(event Collision|EventActorBeginOverlap
  (params (OtherActor :type Actor%20Object%20Reference)))

(event EventTick
  (params (DeltaSeconds :type Float%20%28single-precision%29)))

(event Collision|EventHit
  (params (MyComp :type Primitive%20Component%20Object%20Reference) (Other :type Actor%20Object%20Reference) (OtherComp :type Primitive%20Component%20Object%20Reference) (bSelfMoved :type Boolean) (HitLocation :type Vector :default "0, 0, 0") (HitNormal :type Vector :default "0, 0, 0") (NormalImpulse :type Vector :default "0, 0, 0") (Hit :type Hit%20Result%20Structure%20%28by%20ref%29))
  (Utilities|Casting|CastToBP_PC2_Bullet Other)
  (Math|Integer|CompareInt (Variables|Default|GetnHit) 3
    (:==
      (if (not (Variables|Default|GetBreak))
        (Game|SpawnActorfromClass "/Game/ExplosionFields/ExplosionField.ExplosionField_C" (Math|Conversions|ToTransform(Vector) (Transformation|GetActorLocation)) "Undefined" 0 0)
        (Variables|Default|SetBreak true)
        (switch int (Math|Random|RandomIntegerinRange 0 3)
          (:0
            (bind _returnvalue (Game|SpawnActorfromClass "/Game/Blueprints/WoodenCube_Blueprint.WoodenCube_Blueprint_C" (Math|Conversions|ToTransform(Vector) (Transformation|GetActorLocation)) "Undefined" 0 0))
            (Variables|/Script/GDENG02_PC2.DropBehaviorActorComponent|SetparentActor (Actor|GetComponentbyClass _returnvalue "/Script/GDENG02_PC2.DropBehaviorActorComponent") self))
          (:1
            (bind _returnvalue_2 (Game|SpawnActorfromClass "/Game/Blueprints/RedCylinderDrop.RedCylinderDrop_C" (Math|Conversions|ToTransform(Vector) (Transformation|GetActorLocation)) "Undefined" 0 0))
            (Variables|/Script/GDENG02_PC2.DropBehaviorActorComponent|SetparentActor (Actor|GetComponentbyClass _returnvalue_2 "/Script/GDENG02_PC2.DropBehaviorActorComponent") self))
          (:2
            (bind _returnvalue_3 (Game|SpawnActorfromClass "/Game/Blueprints/OrangeCapsuleDrop.OrangeCapsuleDrop_C" (Math|Conversions|ToTransform(Vector) (Transformation|GetActorLocation)) "Undefined" 0 0))
            (Variables|/Script/GDENG02_PC2.DropBehaviorActorComponent|SetparentActor (Actor|GetComponentbyClass _returnvalue_3 "/Script/GDENG02_PC2.DropBehaviorActorComponent") self))
          (:3
            (bind _returnvalue_4 (Game|SpawnActorfromClass "/Game/Blueprints/YellowConeDrop.YellowConeDrop_C" (Math|Conversions|ToTransform(Vector) (Transformation|GetActorLocation)) "Undefined" 0 0))
            (Variables|/Script/GDENG02_PC2.DropBehaviorActorComponent|SetparentActor (Actor|GetComponentbyClass _returnvalue_4 "/Script/GDENG02_PC2.DropBehaviorActorComponent") self)))))
    (:<
      (Variables|Default|SetnHit (+ (Variables|Default|GetnHit) 1)))))

(fn ConstructionScript)